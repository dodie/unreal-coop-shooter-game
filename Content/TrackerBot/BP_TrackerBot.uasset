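; Tracker bot Blueprint whose graph holds only leftover debug and obsolete logic, with a comment noting a move to C++.
; FindNextPathPoint finds a navigation path to player pawn 0 and draws debug spheres at its waypoints, without moving the bot.
; BeginPlay, Tick and the construction script are empty.
; The call to FindNextPathPoint and the speed-based rolling sound volume update are disconnected and never run.
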(event Custom|FindNextPathPoint
  ;[1 1 1] Debug - plan route to player and draw spheres on the waypoints
  (bind _returnvalue (Class|NavigationSystem|FindPathtoActorSynchronously (Transformation|GetActorLocation) (Game|Player|GetPlayerPawn 0) 5e+01))
  (for _array_element (Variables|/Script/Engine.NavigationPath|GetPathPoints _returnvalue)
    (Rendering|Debug|DrawDebugSphere _array_element 1e+02 12 "(R=1.000000,G=0.070812,B=0.887641,A=1.000000)" 1e+01 2.0)))

(event EventBeginPlay
  ;[1 1 1] Debug - plan route to player and draw spheres on the waypoints
)

(event EventTick
  (params (DeltaSeconds :type Float%20%28single-precision%29))
  ;[1 1 1] Obsolete - now implemented in C++
)

(fn ConstructionScript)