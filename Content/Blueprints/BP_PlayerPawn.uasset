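; BP_PlayerPawn is the player pawn Blueprint, handling the local player's HUD and in-game menu.
; On BeginPlay it waits briefly, working around IsLocallyControlled misreporting on listen servers, then clears existing widgets and adds crosshair, health, score and wave widgets for the locally controlled pawn.
; The OpenMenu action creates the in-game menu above the HUD, shows the cursor and switches player controller 0 to UI-only input.
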(event EventBeginPlay
  ;[1 1 1] Create UI Widgets
  ;;[1 1 1] Workaround: Is locally controlled returns false for server for the firest few ticks
  ;; https://answers.unrealengine.com/questions/713607/is-locally-controlled-returns-false-for-listen-ser.html
  (Utilities|FlowControl|Delay 0.2)
  (if (Pawn|IsLocallyControlled)
    (Utilities|FlowControl|Sequence
      (:then_0
        (Viewport|RemoveAllWidgets))
      (:then_1
        (bind _returnvalue (UserInterface|CreateWidget "/Game/UI/WBP_Crosshair.WBP_Crosshair_C"))
        (UserInterface|Viewport|AddtoViewport _returnvalue 0))
      (:then_2
        (bind _returnvalue_2 (UserInterface|CreateWidget "/Game/UI/WBP_HealthIndicator.WBP_HealthIndicator_C"))
        (UserInterface|Viewport|AddtoViewport _returnvalue_2 0))
      (:then_3
        (bind _returnvalue_3 (UserInterface|CreateWidget "/Game/UI/WBP_ScoreIndicator.WBP_ScoreIndicator_C"))
        (UserInterface|Viewport|AddtoViewport _returnvalue_3 0))
      (:then_4
        (bind _returnvalue_4 (UserInterface|CreateWidget "/Game/UI/WBP_WaveStateFlash.WBP_WaveStateFlash_C"))
        (UserInterface|Viewport|AddtoViewport _returnvalue_4 0))
      (:then_5
        (bind _returnvalue_5 (UserInterface|CreateWidget "/Game/UI/WBP_WaveCountIndicator.WBP_WaveCountIndicator_C"))
        (UserInterface|Viewport|AddtoViewport _returnvalue_5 0)))))

(event Input|ActionEvents|InputActionOpenMenu
  (params (Key :type Key%20Structure))
  (bind _returnvalue (Game|GetPlayerController 0))
  ;[1 1 1] Binding For Menu
  (:Pressed
    (bind _returnvalue_2 (UserInterface|CreateWidget "/Game/UI/WBP_IngameMenu.WBP_IngameMenu_C"))
    (UserInterface|Viewport|AddtoViewport _returnvalue_2 10)
    (Variables|/Script/Engine.PlayerController|SetbShowMouseCursor _returnvalue true)
    (Input|SetInputModeUIOnly _returnvalue 0 "LockAlways")))

(fn ConstructionScript)