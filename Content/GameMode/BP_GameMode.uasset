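; Game mode Blueprint that spawns enemy bots and awards score for kills.
; SpawnNewBot runs an EQS query for a spawn location drawn randomly from the best quarter of results.
; On success, a weighted roll spawns either a tracker bot, favored, or a soldier bot with its behavior tree.
; An OnActorKilled binding adds a point to the killer's SPlayerState when a pawn kills another pawn.
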(event Custom|OnQueryFinishedEvent_Event_0
  (params (QueryInstance :type Env%20Query%20Instance%20Blueprint%20Wrapper%20Object%20Reference) (QueryStatus :type EEnvQueryStatus%20Enum :default "Processing"))
  ;[1 1 1] Wave spawn hooks
  (switch Utilities|FlowControl|Switch|SwitchonEEnvQueryStatus QueryStatus
    (:Success
      (for _array_element (Class|EnvQueryInstanceBlueprintWrapper|GetResultsasLocations QueryInstance)
        (if (<= (Math|Random|RandomFloatinRange 0.0 1e+02) 6e+01)
          (Game|SpawnActorfromClass "/Game/TrackerBot/BP_TrackerBot.BP_TrackerBot_C" (Math|Transform|MakeTransform _array_element) "AlwaysSpawn" 0 0)
          (else
            (AI|SpawnAIFromClass "/Game/SoldierBot/BP_SoldierBot.BP_SoldierBot_C" "/Game/SoldierBot/BT_SoldierBotAI.BT_SoldierBotAI" (Math|Transform|TransformLocation (Math|Transform|MakeTransform _array_element) "0, 0, 0") "0, 0, 0" false)))))))

(event Custom|OnActorKilled_Event_0
  (params (VictimActor :type Actor%20Object%20Reference) (KillerActor :type Actor%20Object%20Reference))
  (Utilities|Casting|CastToPawn VictimActor)
  (bind _aspawn (Utilities|Casting|CastToPawn KillerActor))
  (bind _assplayer_state (Utilities|Casting|CastToSPlayerState (Variables|/Script/Engine.Pawn|GetPlayerState _aspawn)))
  (Class|SPlayerState|AddScore _assplayer_state 1.0))

(event EventSpawnNewBot
  ;[1 1 1] Wave spawn hooks
  (bind _returnvalue (AI|EQS|RunEQSQuery "/Game/GameMode/EQS_FindSpawnLocation.EQS_FindSpawnLocation" self "RandomBest25Pct"))
  (EventDispatchers|AssignOnQueryFinishedEvent _returnvalue (delegate Custom|OnQueryFinishedEvent_Event_0)))

(event EventBeginPlay
  (EventDispatchers|AssignOnActorKilled (delegate Custom|OnActorKilled_Event_0)))

(fn ConstructionScript)